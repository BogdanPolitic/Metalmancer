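; DecideInteractionBP decides which of the player or a targeted metal object moves, and in which direction, for a push or pull interaction.
; DecideWhich casts both actors and compares their Mass, selecting the object as WhichActor if the player is heavier, otherwise the player.
; The other actor becomes OtherActor, and IsPushAction sets the sign of WhichDirection, which is inverted when the player is the selected actor.
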(fn ConstructionScript)

(fn DecideWhich
  (bind _ispushaction (Variables|Default|GetIsPushAction))
  (bind _asinteractable_metal_bp (Utilities|Casting|CastToInteractableMetalBP (Variables|Default|GetTargetedObjectActor)))
  (bind _asthird_person_character (Utilities|Casting|CastToThirdPersonCharacter (Variables|Default|GetPlayerActor)))
  (if (> (Variables|/Game/ThirdPersonBP/Blueprints/ThirdPersonCharacter.ThirdPersonCharacter_C|GetMass _asthird_person_character) (Variables|/Game/MyBlueprints/InteractableMetalBP.InteractableMetalBP_C|GetMass _asinteractable_metal_bp))
    (Variables|Default|SetWhichActor (Variables|Default|GetTargetedObjectActor))
    (Variables|Default|SetOtherActor (Variables|Default|GetPlayerActor))
    (if _ispushaction
      (Variables|Default|SetWhichDirection 1.0)
      (else
        (Variables|Default|SetWhichDirection -1.0)))
    (else
      (Variables|Default|SetWhichActor (Variables|Default|GetPlayerActor))
      (Variables|Default|SetOtherActor (Variables|Default|GetTargetedObjectActor))
      (if _ispushaction
        (Variables|Default|SetWhichDirection -1.0)
        (else
          (Variables|Default|SetWhichDirection 1.0))))))